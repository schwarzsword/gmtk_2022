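; Player-controlled cube pawn that slides across navigable tiles, tumbling down ledges and climbing over blocks.
; Four-direction overlap colliders trigger timeline-driven move and rotate sequences, recursing while no floor is found and snapping rotation to 90 degrees.
; Each roll permutes tracked side variables, and the active side selects the rune mesh.
; Falls cost HP; death or R shatters the cube through a geometry collection and physics fields, then reloads the level.
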(event OnComponentEndOverlap(SCollider)
  (params (OverlappedComponent :type Primitive%20Component%20Object%20Reference) (OtherActor :type Actor%20Object%20Reference) (OtherComp :type Primitive%20Component%20Object%20Reference) (OtherBodyIndex :type Integer))
  (bind _cubecollision (Variables|Default|GetCubeCollision))
  (bind _returnvalue (Transformation|GetWorldLocation _cubecollision))
  ;[1 1 1] Falling
  (if (and (Utilities|NoFloorConnection (Variables|Default|GetSCollider)) (Variables|Default|GetRotationCheckEnabled))
    (Variables|Default|SetRotationCheckEnabled false)
    (CallFunction|LinearMove _returnvalue (- _returnvalue "0,50.000000,0") false)
    (Utilities|FlowControl|Delay (Variables|Default|GetLinearMoveDelay))
    (CallFunction|HandleSFalling)))

(event OnComponentEndOverlap(WCollider)
  (params (OverlappedComponent :type Primitive%20Component%20Object%20Reference) (OtherActor :type Actor%20Object%20Reference) (OtherComp :type Primitive%20Component%20Object%20Reference) (OtherBodyIndex :type Integer))
  (bind _cubecollision (Variables|Default|GetCubeCollision))
  (bind _returnvalue (Transformation|GetWorldLocation _cubecollision))
  ;[1 1 1] Falling
  (if (and (Utilities|NoFloorConnection (Variables|Default|GetWCollider)) (Variables|Default|GetRotationCheckEnabled))
    (Variables|Default|SetRotationCheckEnabled false)
    (CallFunction|LinearMove _returnvalue (- _returnvalue "0,-50.000000,0") false)
    (Utilities|FlowControl|Delay (Variables|Default|GetLinearMoveDelay))
    (CallFunction|HandleWFalling)))

(event OnComponentEndOverlap(ACollider)
  (params (OverlappedComponent :type Primitive%20Component%20Object%20Reference) (OtherActor :type Actor%20Object%20Reference) (OtherComp :type Primitive%20Component%20Object%20Reference) (OtherBodyIndex :type Integer))
  (bind _cubecollision (Variables|Default|GetCubeCollision))
  (bind _returnvalue (Transformation|GetWorldLocation _cubecollision))
  ;[1 1 1] Falling
  (if (and (Utilities|NoFloorConnection (Variables|Default|GetACollider)) (Variables|Default|GetRotationCheckEnabled))
    (Variables|Default|SetRotationCheckEnabled false)
    (CallFunction|LinearMove _returnvalue (- _returnvalue "-50.000000,0.000000,0") false)
    (Utilities|FlowControl|Delay (Variables|Default|GetLinearMoveDelay))
    (CallFunction|HandleAFalling)))

(event OnComponentEndOverlap(DCollider)
  (params (OverlappedComponent :type Primitive%20Component%20Object%20Reference) (OtherActor :type Actor%20Object%20Reference) (OtherComp :type Primitive%20Component%20Object%20Reference) (OtherBodyIndex :type Integer))
  (bind _cubecollision (Variables|Default|GetCubeCollision))
  (bind _returnvalue (Transformation|GetWorldLocation _cubecollision))
  ;[1 1 1] Falling
  (if (and (Utilities|NoFloorConnection (Variables|Default|GetDCollider)) (Variables|Default|GetRotationCheckEnabled))
    (Variables|Default|SetRotationCheckEnabled false)
    (CallFunction|LinearMove _returnvalue (- _returnvalue "50.000000,0.000000,0") false)
    (Utilities|FlowControl|Delay (Variables|Default|GetLinearMoveDelay))
    (CallFunction|HandleDFalling)))

(event OnComponentBeginOverlap(DownColliderD)
  (params (OverlappedComponent :type Primitive%20Component%20Object%20Reference) (OtherActor :type Actor%20Object%20Reference) (OtherComp :type Primitive%20Component%20Object%20Reference) (OtherBodyIndex :type Integer) (bFromSweep :type Boolean) (SweepResult :type Hit%20Result%20Structure%20%28by%20ref%29))
  ;[1 1 1] Climbing
  (Utilities|Casting|CastToBP_NavigableTile OtherActor)
  (if (and (Variables|Default|GetRotationCheckEnabled) (Utilities|NoConnection (Variables|Default|GetUpD)))
    (Variables|Default|SetRotationCheckEnabled false)
    (CallFunction|HandleDCLimb)))

(event OnComponentBeginOverlap(DownColliderS)
  (params (OverlappedComponent :type Primitive%20Component%20Object%20Reference) (OtherActor :type Actor%20Object%20Reference) (OtherComp :type Primitive%20Component%20Object%20Reference) (OtherBodyIndex :type Integer) (bFromSweep :type Boolean) (SweepResult :type Hit%20Result%20Structure%20%28by%20ref%29))
  ;[1 1 1] Climbing
  (Utilities|Casting|CastToBP_NavigableTile OtherActor)
  (if (and (Variables|Default|GetRotationCheckEnabled) (Utilities|NoConnection (Variables|Default|GetUpS)))
    (Variables|Default|SetRotationCheckEnabled false)
    (CallFunction|HandleSClimb)))

(event OnComponentBeginOverlap(DownColliderW)
  (params (OverlappedComponent :type Primitive%20Component%20Object%20Reference) (OtherActor :type Actor%20Object%20Reference) (OtherComp :type Primitive%20Component%20Object%20Reference) (OtherBodyIndex :type Integer) (bFromSweep :type Boolean) (SweepResult :type Hit%20Result%20Structure%20%28by%20ref%29))
  ;[1 1 1] Climbing
  (Utilities|Casting|CastToBP_NavigableTile OtherActor)
  (if (and (Variables|Default|GetRotationCheckEnabled) (Utilities|NoConnection (Variables|Default|GetUpW)))
    (Variables|Default|SetRotationCheckEnabled false)
    (CallFunction|HandleWClimb)))

(event OnComponentBeginOverlap(DownColliderA)
  (params (OverlappedComponent :type Primitive%20Component%20Object%20Reference) (OtherActor :type Actor%20Object%20Reference) (OtherComp :type Primitive%20Component%20Object%20Reference) (OtherBodyIndex :type Integer) (bFromSweep :type Boolean) (SweepResult :type Hit%20Result%20Structure%20%28by%20ref%29))
  ;[1 1 1] Climbing
  (Utilities|Casting|CastToBP_NavigableTile OtherActor)
  (if (and (Variables|Default|GetRotationCheckEnabled) (Utilities|NoConnection (Variables|Default|GetUpA)))
    (Variables|Default|SetRotationCheckEnabled false)
    (CallFunction|HandleAClimb)))

(event Custom|HandleWFalling
  ;[1 1 1] Falling
  (CallFunction|Rotate (- (Transformation|GetWorldLocation (Variables|Default|GetCubeCollision)) "0,0.000000,100.000000") (Math|Rotator|MakeRotator 9e+01 0.0 0.0) false)
  (Utilities|FlowControl|Delay (Variables|Default|GetRotationDelay))
  (CallFunction|RotateSidesW)
  (if (Utilities|NoFloorConnection (Variables|Default|GetWCollider))
    (CallFunction|HandleWFalling)
    (else
      (Variables|Default|SetRotationCheckEnabled true)
      (Default|CallOnFall))))

(event Custom|HandleDCLimb
  ;[1 1 1] Climbing
  (CallFunction|Rotate (+ (Transformation|GetWorldLocation (Variables|Default|GetCubeCollision)) "0,0,100.000000") "90.000000, 0,0.000000" true)
  (Utilities|FlowControl|Delay (Variables|Default|GetRotationDelay))
  (CallFunction|RotateSidesD)
  (CallFunction|Rotate (+ (Transformation|GetWorldLocation (Variables|Default|GetCubeCollision)) "-70.000000,0.000000,0") "90.000000, 0,0.000000" true)
  (Utilities|FlowControl|Delay (Variables|Default|GetRotationDelay))
  (CallFunction|RotateSidesD)
  (Variables|Default|SetRotationCheckEnabled true))

(event Custom|HandleSClimb
  ;[1 1 1] Climbing
  (CallFunction|Rotate (+ (Transformation|GetWorldLocation (Variables|Default|GetCubeCollision)) "0,0,100.000000") "0, 0,-90.000000" true)
  (Utilities|FlowControl|Delay (Variables|Default|GetRotationDelay))
  (CallFunction|RotateSidesS)
  (CallFunction|Rotate (+ (Transformation|GetWorldLocation (Variables|Default|GetCubeCollision)) "0,-70.000000,0") "0, 0,-90.000000" true)
  (Utilities|FlowControl|Delay (Variables|Default|GetRotationDelay))
  (CallFunction|RotateSidesS)
  (Variables|Default|SetRotationCheckEnabled true))

(event Custom|HandleWClimb
  ;[1 1 1] Climbing
  (CallFunction|Rotate (+ (Transformation|GetWorldLocation (Variables|Default|GetCubeCollision)) "0,0,100.000000") "0, 0,90.000000" true)
  (Utilities|FlowControl|Delay (Variables|Default|GetRotationDelay))
  (CallFunction|RotateSidesW)
  (CallFunction|Rotate (+ (Transformation|GetWorldLocation (Variables|Default|GetCubeCollision)) "0,70.000000,0") "0, 0,90.000000" true)
  (Utilities|FlowControl|Delay (Variables|Default|GetRotationDelay))
  (CallFunction|RotateSidesW)
  (Variables|Default|SetRotationCheckEnabled true))

(event Custom|HandleAClimb
  ;[1 1 1] Climbing
  (CallFunction|Rotate (+ (Transformation|GetWorldLocation (Variables|Default|GetCubeCollision)) "0,0,100.000000") "-90.000000, 0,0.000000" true)
  (Utilities|FlowControl|Delay (Variables|Default|GetRotationDelay))
  (CallFunction|RotateSidesA)
  (CallFunction|Rotate (+ (Transformation|GetWorldLocation (Variables|Default|GetCubeCollision)) "70.000000,0.000000,0") "-90.000000, 0,0.000000" true)
  (Utilities|FlowControl|Delay (Variables|Default|GetRotationDelay))
  (CallFunction|RotateSidesA)
  (Variables|Default|SetRotationCheckEnabled true))

(event Custom|Fall
  (Default|FunctionRemoveHP (Variables|Components|GetBP_CubeHP))
  (Niagara|SpawnSystematLocation "/Game/FX/FlipBook/NS_CubeFall.NS_CubeFall" (- (Transformation|GetWorldLocation (Variables|Default|GetCubeCollision)) "0,0,50.000000") "0, 0, 0" "10.000000,10.000000,10.000000")
  (CallFunction|DoCameraShake))

(event Custom|Rotate
  (params (TargetLocation :type Vector) (TargetRotation :type Rotator) (Up? :type Boolean))
  (bind _returnvalue (/ 1.0 3e+01))
  (bind _cube (Variables|Components|GetCube))
  (bind _returnvalue_2 (Transformation|GetWorldRotation _cube))
  (bind _returnvalue_3 (* TargetRotation _returnvalue))
  (bind (_roll _pitch _yaw) (Math|Rotator|BreakRotator _returnvalue_3))
  ;[1 1 1] LinearRotate
  (Variables|Default|SetSomeRotation "0, 0, 0")
  (bind _output_get (Variables|Default|SetStartFallingPosition (Transformation|GetWorldLocation (Variables|Components|GetCube))))
  (bind _newtrack_0 (Timeline|Falling PlayFromStart)
    (:Update
      (Transformation|SetWorldLocation (Variables|Default|GetCubeCollision) (Math|Vector|Lerp(Vector) _output_get TargetLocation _newtrack_0) false false)
      (Variables|Default|SetSomeRotation (Math|Rotator|MakeRotator (+ _roll (.roll (Variables|Default|GetSomeRotation))) (+ _pitch (.pitch (Variables|Default|GetSomeRotation))) (+ _yaw (.yaw (Variables|Default|GetSomeRotation)))))
      (if (not (or (and (Math|Boolean|ORBoolean (> (.roll (Variables|Default|GetSomeRotation)) 9e+01) (< (.roll (Variables|Default|GetSomeRotation)) -9e+01) (> (.pitch (Variables|Default|GetSomeRotation)) 9e+01) (< (.pitch (Variables|Default|GetSomeRotation)) -9e+01) (> (.yaw (Variables|Default|GetSomeRotation)) 9e+01) (< (.yaw (Variables|Default|GetSomeRotation)) -9e+01)) (not Up?)) (and (Math|Boolean|ORBoolean (> (.roll (Variables|Default|GetSomeRotation)) 1.8e+02) (< (.roll (Variables|Default|GetSomeRotation)) -1.8e+02) (> (.pitch (Variables|Default|GetSomeRotation)) 1.8e+02) (< (.pitch (Variables|Default|GetSomeRotation)) -1.8e+02) (> (.yaw (Variables|Default|GetSomeRotation)) 1.8e+02) (< (.yaw (Variables|Default|GetSomeRotation)) -1.8e+02)) Up?)))
        (Transformation|AddWorldRotation (Variables|Components|GetCube) _returnvalue_3 false false)))
    (:Finished
      (Transformation|SetWorldRotation _cube (Math|Rotator|MakeRotator (Utilities|Clamp90 (.roll _returnvalue_2)) (Utilities|Clamp90 (.pitch _returnvalue_2)) (Utilities|Clamp90 (.yaw _returnvalue_2))) false false))))

(event Custom|HandleAFalling
  ;[1 1 1] Falling
  (CallFunction|Rotate (- (Transformation|GetWorldLocation (Variables|Default|GetCubeCollision)) "0.000000,0.000000,100.000000") (Math|Rotator|MakeRotator 0.0 -9e+01 0.0) false)
  (Utilities|FlowControl|Delay (Variables|Default|GetRotationDelay))
  (CallFunction|RotateSidesA)
  (if (Utilities|NoFloorConnection (Variables|Default|GetACollider))
    (CallFunction|HandleAFalling)
    (else
      (Variables|Default|SetRotationCheckEnabled true)
      (Default|CallOnFall))))

(event Custom|OnDeath
  ;[1 1 1] Init
  (CallFunction|HandleDeath)
  (Utilities|FlowControl|Delay 2.0)
  (bind _returnvalue (UserInterface|CreateWidget "/Game/UI/WBP_LevelLoading.WBP_LevelLoading_C"))
  (UserInterface|Viewport|AddtoViewport _returnvalue 1)
  (Utilities|FlowControl|Delay 0.8)
  (CallFunction|RestartLevel))

(event Custom|HandleDFalling
  ;[1 1 1] Falling
  (CallFunction|Rotate (- (Transformation|GetWorldLocation (Variables|Default|GetCubeCollision)) "0.000000,0.000000,100.000000") (Math|Rotator|MakeRotator 0.0 9e+01 0.0) false)
  (Utilities|FlowControl|Delay (Variables|Default|GetRotationDelay))
  (CallFunction|RotateSidesD)
  (if (Utilities|NoFloorConnection (Variables|Default|GetDCollider))
    (CallFunction|HandleDFalling)
    (else
      (Variables|Default|SetRotationCheckEnabled true)
      (Default|CallOnFall))))

(event Custom|LinearMove
  (params (StartPosition :type Vector) (EndPosition :type Vector) (Slow :type Boolean))
  (bind _cubecollision (Variables|Default|GetCubeCollision))
  ;[1 1 1] LinearMove
  (bind _output_get (Variables|Default|SetStartFallingPosition StartPosition))
  (if Slow
    (bind _newtrack_0 (Timeline|Timeline_1 PlayFromStart)
      (:Update
        (Transformation|SetWorldLocation _cubecollision (Math|Vector|Lerp(Vector) _output_get EndPosition _newtrack_0) false false)))
    (else
      (bind _newtrack_0_2 (Timeline|Timeline_0 PlayFromStart)
        (:Update
          (Transformation|SetWorldLocation _cubecollision (Math|Vector|Lerp(Vector) _output_get EndPosition _newtrack_0_2) false false))))))

(event Custom|HandleSFalling
  ;[1 1 1] Falling
  (CallFunction|Rotate (- (Transformation|GetWorldLocation (Variables|Default|GetCubeCollision)) "0,0.000000,100.000000") (Math|Rotator|MakeRotator -9e+01 0.0 0.0) false)
  (Utilities|FlowControl|Delay (Variables|Default|GetRotationDelay))
  (CallFunction|RotateSidesS)
  (if (Utilities|NoFloorConnection (Variables|Default|GetSCollider))
    (CallFunction|HandleSFalling)
    (else
      (Variables|Default|SetRotationCheckEnabled true)
      (Default|CallOnFall))))

(event Custom|OnActiveSideChange_Event
  (params (NewParam :type E_CubeSides%20Enum :default "NewEnumerator0"))
  ;[1 1 1] Init
  (Utilities|SetRuneMesh NewParam))

(event EventBeginPlay
  ;[1 1 1] Init
  (EventDispatchers|BindEventtoOnActiveSideChange (delegate Custom|OnActiveSideChange_Event))
  (Utilities|SetRuneMesh (Variables|Default|GetActiveSide)
    (:out
      (EventDispatchers|BindEventtoDeath (Variables|Components|GetBP_CubeHP) (delegate Custom|OnDeath))
      (EventDispatchers|BindEventtoOnFall (delegate Custom|Fall)))))

(event Input|AxisEvents|InputAxisMoveForward
  (params (AxisValue :type Float%20%28single-precision%29))
  (bind _moveparticles (Variables|Default|GetMoveParticles))
  ;[1 1 1] Comment
  (if (Variables|Default|GetRotationCheckEnabled)
    (Pawn|Input|AddMovementInput "0,1.000000, 0" (.x (/ (Math|Vector|Normalize (Math|Vector|MakeVector AxisValue (stale Input|AxisEvents|InputAxisMoveRight AxisValue) 0.0)) "2.000000,2.000000,2.000000")) false)
    (Components|Activation|Activate _moveparticles false)
    (Utilities|FlowControl|RetriggerableDelay 0.2)
    (Components|Activation|Deactivate _moveparticles)))

(event Input|AxisEvents|InputAxisMoveRight
  (params (AxisValue :type Float%20%28single-precision%29))
  (bind _moveparticles (Variables|Default|GetMoveParticles))
  ;[1 1 1] Comment
  (if (Variables|Default|GetRotationCheckEnabled)
    (Pawn|Input|AddMovementInput "-1.000000, 0, 0" (.y (/ (Math|Vector|Normalize (Math|Vector|MakeVector (stale Input|AxisEvents|InputAxisMoveForward AxisValue) AxisValue 0.0)) "2.000000,2.000000,2.000000")) false)
    (Components|Activation|Activate _moveparticles false)
    (Utilities|FlowControl|RetriggerableDelay 0.2)
    (Components|Activation|Deactivate _moveparticles)))

(event Input|KeyboardEvents|R
  (params (Key :type Key%20Structure :default "None")))

(event Input|KeyboardEvents|R
  (params (Key :type Key%20Structure :default "None"))
  (:Pressed
    ;[1 1 1] Init
    (CallFunction|HandleDeath)
    (Utilities|FlowControl|Delay 2.0)
    (bind _returnvalue (UserInterface|CreateWidget "/Game/UI/WBP_LevelLoading.WBP_LevelLoading_C"))
    (UserInterface|Viewport|AddtoViewport _returnvalue 1)
    (Utilities|FlowControl|Delay 0.8)
    (CallFunction|RestartLevel)))

(fn ConstructionScript
  (Transformation|SetActorRotation "0,-90.000000, 0"))

(fn HandleDeath
  (bind _cubecollision (Variables|Default|GetCubeCollision))
  (bind _staticmesh (Variables|Default|GetStaticMesh))
  (bind _returnvalue (Transformation|GetRelativeTransform _staticmesh))
  (Variables|Default|SetStartFallingPosition (Transformation|GetWorldLocation _cubecollision))
  (Development|SetHiddeninGame _cubecollision true true)
  (Collision|SetCollisionResponsetoAllChannels _cubecollision "ECR_Ignore")
  (AddComponent|AddGeometryCollectionComponent false (Math|Transform|MakeTransform (.location _returnvalue) (.rotation _returnvalue) "1.000000,1.000000,1.000000"))
  (bind _returnvalue_2 (AddComponent|AddRadialFalloff))
  (bind _returnvalue_3 (AddComponent|AddRadialVector))
  (bind _returnvalue_4 (AddComponent|AddFieldSystemComponent false))
  (Class|FieldSystemComponent|ApplyPhysicsField _returnvalue_4 true "Field_ExternalClusterStrain" 0 (Field|SetRadialFalloff _returnvalue_2 (LocalVariables|GetForce) 0.0 1.0 0.0 (LocalVariables|GetRadius) (Variables|Default|GetStartFallingPosition) "Field_FallOff_None"))
  (Class|FieldSystemComponent|ApplyPhysicsField _returnvalue_4 true "Field_LinearForce" 0 (Field|SetRadialVector _returnvalue_3 (LocalVariables|GetForce) (Variables|Default|GetStartFallingPosition))))

(fn RotateSidesW
  (Variables|Default|SetTemp (Variables|Default|GetActiveSide))
  (bind _output_get (Variables|Default|SetActiveSide (Variables|Default|GetSSide)))
  (Variables|Default|SetSSide (Variables|Default|GetDownSide))
  (Variables|Default|SetDownSide (Variables|Default|GetWSide))
  (Variables|Default|SetWSide (Variables|Default|GetTemp))
  (Default|CallOnActiveSideChange _output_get))

(fn RotateSidesS
  (Variables|Default|SetTemp (Variables|Default|GetActiveSide))
  (bind _output_get (Variables|Default|SetActiveSide (Variables|Default|GetWSide)))
  (Variables|Default|SetWSide (Variables|Default|GetDownSide))
  (Variables|Default|SetDownSide (Variables|Default|GetSSide))
  (Variables|Default|SetSSide (Variables|Default|GetTemp))
  (Default|CallOnActiveSideChange _output_get))

(fn RotateSidesA
  (Variables|Default|SetTemp (Variables|Default|GetActiveSide))
  (bind _output_get (Variables|Default|SetActiveSide (Variables|Default|GetDSide)))
  (Variables|Default|SetDSide (Variables|Default|GetDownSide))
  (Variables|Default|SetDownSide (Variables|Default|GetASide))
  (Variables|Default|SetASide (Variables|Default|GetTemp))
  (Default|CallOnActiveSideChange _output_get))

(fn RotateSidesD
  (Variables|Default|SetTemp (Variables|Default|GetActiveSide))
  (bind _output_get (Variables|Default|SetActiveSide (Variables|Default|GetASide)))
  (Variables|Default|SetASide (Variables|Default|GetDownSide))
  (Variables|Default|SetDownSide (Variables|Default|GetDSide))
  (Variables|Default|SetDSide (Variables|Default|GetTemp))
  (Default|CallOnActiveSideChange _output_get))

(fn RestartLevel
  (bind _returnvalue (Game|GetCurrentLevelName true))
  (Game|OpenLevel(byName) (Utilities|String|StringToName _returnvalue)))