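; BP_Plumb is a placeable "plum" mesh actor with dirt, stone, grass and snow variants, each in a big or small size.
; The Construction Script picks the static mesh from TypePlum and IsBig, falling back to dirt for unhandled types.
; It also gives the mesh a random yaw on every construction to vary copies.
; The Event Graph holds only disabled stub events, so it adds no runtime logic.
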(event EventBeginPlay)

(event Collision|EventActorBeginOverlap
  (params (OtherActor :type Actor%20Object%20Reference)))

(event EventTick
  (params (DeltaSeconds :type Float%20%28single-precision%29)))

(fn ConstructionScript
  (bind _staticmesh (Variables|Default|GetStaticMesh))
  (bind _isbig (Variables|Default|GetisBig))
  (Transformation|SetRelativeRotation (Variables|Default|GetStaticMesh) (Math|Rotator|MakeRotator 0.0 0.0 (Math|Random|RandomFloatinRange 0.0 3.6e+02)) false false)
  (switch int (Variables|Default|GetTypePlum)
    (:Default
      (if _isbig :!label _label
        (Components|StaticMesh|SetStaticMesh _staticmesh "/Game/Static/plum_dirt_b.plum_dirt_b")
        (else
          (Components|StaticMesh|SetStaticMesh _staticmesh "/Game/Static/plum_dirt_s.plum_dirt_s"))))
    (:0
      (goto _label))
    (:1
      (if _isbig
        (Components|StaticMesh|SetStaticMesh _staticmesh "/Game/Static/plum_stone_b.plum_stone_b")
        (else
          (Components|StaticMesh|SetStaticMesh _staticmesh "/Game/Static/plum_stone_s.plum_stone_s"))))
    (:2
      (if _isbig
        (Components|StaticMesh|SetStaticMesh _staticmesh "/Game/Static/plum_grass_b.plum_grass_b")
        (else
          (Components|StaticMesh|SetStaticMesh _staticmesh "/Game/Static/plum_grass_s.plum_grass_s"))))
    (:3
      (if _isbig
        (Components|StaticMesh|SetStaticMesh _staticmesh "/Game/Static/plum_snow_b.plum_snow_b")
        (else
          (Components|StaticMesh|SetStaticMesh _staticmesh "/Game/Static/plum_snow_s.plum_snow_s"))))))