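; Level-exit door actor that opens when BP_PlayerCube overlaps it with the required side active, then loads the next level.
; The construction script sets the lock rune, light and Niagara color from NeedThisSide.
; A DoOnce-gated match halts the cube, lerps it into place via timeline, enables physics, swings the doors and drops floor collision.
; The next level name derives from the current "L" number, falling back to MainMenu from 19 onward.
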(event OnComponentBeginOverlap(CollisionBox)
  (params (OverlappedComponent :type Primitive%20Component%20Object%20Reference) (OtherActor :type Actor%20Object%20Reference) (OtherComp :type Primitive%20Component%20Object%20Reference) (OtherBodyIndex :type Integer) (bFromSweep :type Boolean) (SweepResult :type Hit%20Result%20Structure%20%28by%20ref%29))
  ;[1 1 1] Сравниваем значение на кубе и нужное, если соответствует - запускаем анимацию перехода на новый уровень
  (Utilities|FlowControl|DoOnce false
    (:Completed
      (bind _asbp_player_cube (Utilities|Casting|CastToBP_PlayerCube OtherActor))
      (Variables|Default|SetAs%20BP%20Player%20Cube _asbp_player_cube)
      (if (Utilities|Enum|Equal(Enum) (Variables|/Game/Blueprints/Characters/BP_PlayerCube.BP_PlayerCube_C|GetActiveSide _asbp_player_cube) (Variables|Default|GetNeedThisSide))
        (Variables|/Game/Blueprints/Characters/BP_PlayerCube.BP_PlayerCube_C|SetRotationCheckEnabled _asbp_player_cube false)
        (Variables|/Script/Engine.FloatingPawnMovement|SetMaxSpeed (Variables|/Game/Blueprints/Characters/BP_PlayerCube.BP_PlayerCube_C|GetFloatingPawnMovement _asbp_player_cube) 0.0)
        (Components|Activation|Activate (Variables|Default|GetNiagara) false)
        (Rendering|SetVisibility (Variables|Default|GetLock) false false)
        (Components|Movement|StopMovementImmediately (Variables|/Game/Blueprints/Characters/BP_PlayerCube.BP_PlayerCube_C|GetFloatingPawnMovement _asbp_player_cube))
        (Audio|PlaySound2D "/Game/Music/Win.Win" 1.0 1.0 0.0 0 0)
        (Variables|Default|Setcur_point (Transformation|GetActorLocation (Variables|Default|GetAs%20BP%20Player%20Cube)))
        (bind _newtrack_0 (Timeline|Timeline_0 PlayFromStart)
          (:Update
            (Transformation|SetActorLocation (Variables|Default|GetAs%20BP%20Player%20Cube) (Math|Vector|Lerp(Vector) (Variables|Default|Getcur_point) (+ (Variables|Default|Getpoint) (Transformation|GetActorLocation)) _newtrack_0) false true))
          (:Finished
            (Physics|SetSimulatePhysics (Variables|/Game/Blueprints/Characters/BP_PlayerCube.BP_PlayerCube_C|GetCubeCollision _asbp_player_cube) true)
            (CallFunction|EventOpenDoor)))))))

(event Custom|Event_OpenDoor
  ;[1 1 1] Открываем ворота и позволяем кубу упасть
  (bind (_direction _door_1 _door_2) (Timeline|OpenDoor Play)
    (:Update
      (Transformation|SetRelativeRotation (Variables|Default|GetPoint_1) (Math|Rotator|MakeRotator 0.0 _door_1 0.0) false false)
      (Transformation|SetRelativeRotation (Variables|Default|GetPoint_2) (Math|Rotator|MakeRotator 0.0 _door_2 0.0) false false))
    (:Finished
      (Collision|SetCollisionEnabled (Variables|Default|GetFloorCollision) "NoCollision")
      (Utilities|FlowControl|Delay 1.0)
      (CallFunction|EventNewLevelOpen)
      (Audio|PlaySound2D "/Game/Music/Win4.Win4" 1.0 1.0 0.0 0 0))))

(event Custom|Event_NewLevelOpen
  ;[1 1 1] Открываем новый уровень
  (bind _returnvalue (Game|GetCurrentLevelName true))
  (if (< (Math|Conversions|ToInteger(Byte) (Utilities|String|Right _returnvalue (- (Utilities|String|Len _returnvalue) 1))) 19)
    (bind _returnvalue_2 (UserInterface|CreateWidget "/Game/UI/WBP_LevelLoading.WBP_LevelLoading_C"))
    (UserInterface|Viewport|AddtoViewport _returnvalue_2 1)
    (Utilities|FlowControl|Delay 3.5)
    (Game|OpenLevel(byName) (Utilities|String|StringToName (Utilities|String|Append "L" (Utilities|String|ToString(Integer) (+ (Math|Conversions|ToInteger(Byte) (Utilities|String|Right _returnvalue (- (Utilities|String|Len _returnvalue) 1))) 1)))))
    (else
      (Game|OpenLevel(byName) "MainMenu"))))

(fn ConstructionScript
  (bind _lock (Variables|Default|GetLock))
  (Transformation|SetRelativeRotation (Variables|Default|GetSpringArm) (Math|Rotator|MakeRotator 0.0 0.0 (Variables|Default|GetFlagRotator)) false false)
  (Transformation|SetRelativeRotation (Variables|Default|GetLock) (Math|Rotator|MakeRotator 0.0 0.0 (Variables|Default|GetRuneRotator)) false false)
  (switch Utilities|FlowControl|Switch|SwitchonE_CubeSides (Variables|Default|GetNeedThisSide)
    (:NewEnumerator0
      (Components|StaticMesh|SetStaticMesh _lock "/Game/Static/rune_lock_1.rune_lock_1")
      (Rendering|Components|Light|SetLightColor (Variables|Default|GetPointLight) "(R=1.000000,G=0.841131,B=0.000000,A=1.000000)" true)
      (Effects|Components|ParticleSystem|SetColorParameter (Variables|Default|GetNiagara) "Color" "(R=1.000000,G=0.839216,B=0.000000,A=1.000000)"))
    (:NewEnumerator1
      (Components|StaticMesh|SetStaticMesh _lock "/Game/Static/rune_lock_2.rune_lock_2")
      (Rendering|Components|Light|SetLightColor (Variables|Default|GetPointLight) "(R=1.000000,G=0.000000,B=0.874510,A=1.000000)" true)
      (Effects|Components|ParticleSystem|SetColorParameter (Variables|Default|GetNiagara) "Color" "(R=1.000000,G=0.000000,B=0.874510,A=1.000000)"))
    (:NewEnumerator2
      (Components|StaticMesh|SetStaticMesh _lock "/Game/Static/rune_lock_3.rune_lock_3")
      (Rendering|Components|Light|SetLightColor (Variables|Default|GetPointLight) "(R=1.000000,G=0.043137,B=0.000000,A=1.000000)" true)
      (Effects|Components|ParticleSystem|SetColorParameter (Variables|Default|GetNiagara) "Color" "(R=1.000000,G=0.043137,B=0.000000,A=1.000000)"))
    (:NewEnumerator3
      (Components|StaticMesh|SetStaticMesh _lock "/Game/Static/rune_lock_4.rune_lock_4")
      (Rendering|Components|Light|SetLightColor (Variables|Default|GetPointLight) "(R=0.000000,G=1.000000,B=0.035294,A=1.000000)" true)
      (Effects|Components|ParticleSystem|SetColorParameter (Variables|Default|GetNiagara) "Color" "(R=0.000000,G=1.000000,B=0.035294,A=1.000000)"))
    (:NewEnumerator4
      (Components|StaticMesh|SetStaticMesh _lock "/Game/Static/rune_lock_5.rune_lock_5")
      (Rendering|Components|Light|SetLightColor (Variables|Default|GetPointLight) "(R=1.000000,G=1.000000,B=1.000000,A=1.000000)" true)
      (Effects|Components|ParticleSystem|SetColorParameter (Variables|Default|GetNiagara) "Color" "(R=1.000000,G=1.000000,B=1.000000,A=1.000000)"))
    (:NewEnumerator5
      (Components|StaticMesh|SetStaticMesh _lock "/Game/Static/rune_lock_6.rune_lock_6")
      (Rendering|Components|Light|SetLightColor (Variables|Default|GetPointLight) "(R=0.000000,G=0.458824,B=1.000000,A=1.000000)" true)
      (Effects|Components|ParticleSystem|SetColorParameter (Variables|Default|GetNiagara) "Color" "(R=0.000000,G=0.458824,B=1.000000,A=1.000000)"))))