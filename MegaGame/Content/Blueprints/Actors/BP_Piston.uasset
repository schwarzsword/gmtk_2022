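; Piston actor whose head extends or retracts along its up vector when a matching trigger value toggles its activated state, and extends at BeginPlay if already active.
; PullHeadUp and PullHeadDown set a signed travel distance and limit, then play or reverse a timeline.
; Timeline updates step the head by world location, using a signed axis code from GetPullDirection to stop at that limit.
; A looping self-toggle timer is left unconnected.
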(event Custom|PullHeadDown
  (bind _head (Variables|Default|Gethead))
  (bind _head_2 (Variables|Default|Gethead))
  (bind _returnvalue (Math|Vector|GetUpVector _head))
  (Variables|Default|SetdirectionMultiplier -1e+02)
  (Variables|Default|SetMoveLimit (+ (Transformation|GetWorldLocation _head) (* _returnvalue (Variables|Default|GetdirectionMultiplier))))
  (bind _direction (CallFunction|GetPullDirection _returnvalue))
  (Variables|Default|SetDirection (* _direction (Math|Float|Sign(Float) (Variables|Default|GetdirectionMultiplier))))
  (if (> (Variables|Default|GetdirectionMultiplier) 0.0)
    (bind _newtrack_0 (Timeline|Timeline_0 Play)
      (:Update
        (switch int (Math|Float|Round (Variables|Default|GetDirection))
          (:-3
            (if (>= (.z (+ (Transformation|GetWorldLocation _head_2) (* (* (Math|Vector|GetUpVector _head_2) (Variables|Default|GetdirectionMultiplier)) _newtrack_0))) (.z (Variables|Default|GetMoveLimit)))
              (Transformation|SetWorldLocation _head_2 (Math|Vector|MakeVector (.x (+ (Transformation|GetWorldLocation _head_2) (* (* (Math|Vector|GetUpVector _head_2) (Variables|Default|GetdirectionMultiplier)) _newtrack_0))) (.y (+ (Transformation|GetWorldLocation _head_2) (* (* (Math|Vector|GetUpVector _head_2) (Variables|Default|GetdirectionMultiplier)) _newtrack_0))) (.z (+ (Transformation|GetWorldLocation _head_2) (* (* (Math|Vector|GetUpVector _head_2) (Variables|Default|GetdirectionMultiplier)) _newtrack_0)))) false false :!label _label)))
          (:-2
            (if (>= (.y (+ (Transformation|GetWorldLocation _head_2) (* (* (Math|Vector|GetUpVector _head_2) (Variables|Default|GetdirectionMultiplier)) _newtrack_0))) (.y (Variables|Default|GetMoveLimit)))
              (goto _label)))
          (:-1
            (if (>= (.x (+ (Transformation|GetWorldLocation _head_2) (* (* (Math|Vector|GetUpVector _head_2) (Variables|Default|GetdirectionMultiplier)) _newtrack_0))) (.x (Variables|Default|GetMoveLimit)))
              (goto _label)))
          (:1
            (if (<= (.x (+ (Transformation|GetWorldLocation _head_2) (* (* (Math|Vector|GetUpVector _head_2) (Variables|Default|GetdirectionMultiplier)) _newtrack_0))) (.x (Variables|Default|GetMoveLimit)))
              (goto _label)))
          (:2
            (if (<= (.y (+ (Transformation|GetWorldLocation _head_2) (* (* (Math|Vector|GetUpVector _head_2) (Variables|Default|GetdirectionMultiplier)) _newtrack_0))) (.y (Variables|Default|GetMoveLimit)))
              (goto _label)))
          (:3
            (if (<= (.z (+ (Transformation|GetWorldLocation _head_2) (* (* (Math|Vector|GetUpVector _head_2) (Variables|Default|GetdirectionMultiplier)) _newtrack_0))) (.z (Variables|Default|GetMoveLimit)))
              (goto _label))))))
    (else
      (Timeline|Timeline_0 Reverse))))

(event Custom|PullHeadUp
  (bind _head (Variables|Default|Gethead))
  (bind _head_2 (Variables|Default|Gethead))
  (bind _returnvalue (Math|Vector|GetUpVector _head))
  (Variables|Default|SetdirectionMultiplier 1e+02)
  (Variables|Default|SetMoveLimit (+ (Transformation|GetWorldLocation _head) (* _returnvalue (Variables|Default|GetdirectionMultiplier))))
  (bind _direction (CallFunction|GetPullDirection _returnvalue))
  (Variables|Default|SetDirection (* _direction (Math|Float|Sign(Float) (Variables|Default|GetdirectionMultiplier))))
  (if (> (Variables|Default|GetdirectionMultiplier) 0.0)
    (bind _newtrack_0 (Timeline|Timeline_0 Play)
      (:Update
        (switch int (Math|Float|Round (Variables|Default|GetDirection))
          (:-3
            (if (>= (.z (+ (Transformation|GetWorldLocation _head_2) (* (* (Math|Vector|GetUpVector _head_2) (Variables|Default|GetdirectionMultiplier)) _newtrack_0))) (.z (Variables|Default|GetMoveLimit)))
              (Transformation|SetWorldLocation _head_2 (Math|Vector|MakeVector (.x (+ (Transformation|GetWorldLocation _head_2) (* (* (Math|Vector|GetUpVector _head_2) (Variables|Default|GetdirectionMultiplier)) _newtrack_0))) (.y (+ (Transformation|GetWorldLocation _head_2) (* (* (Math|Vector|GetUpVector _head_2) (Variables|Default|GetdirectionMultiplier)) _newtrack_0))) (.z (+ (Transformation|GetWorldLocation _head_2) (* (* (Math|Vector|GetUpVector _head_2) (Variables|Default|GetdirectionMultiplier)) _newtrack_0)))) false false :!label _label)))
          (:-2
            (if (>= (.y (+ (Transformation|GetWorldLocation _head_2) (* (* (Math|Vector|GetUpVector _head_2) (Variables|Default|GetdirectionMultiplier)) _newtrack_0))) (.y (Variables|Default|GetMoveLimit)))
              (goto _label)))
          (:-1
            (if (>= (.x (+ (Transformation|GetWorldLocation _head_2) (* (* (Math|Vector|GetUpVector _head_2) (Variables|Default|GetdirectionMultiplier)) _newtrack_0))) (.x (Variables|Default|GetMoveLimit)))
              (goto _label)))
          (:1
            (if (<= (.x (+ (Transformation|GetWorldLocation _head_2) (* (* (Math|Vector|GetUpVector _head_2) (Variables|Default|GetdirectionMultiplier)) _newtrack_0))) (.x (Variables|Default|GetMoveLimit)))
              (goto _label)))
          (:2
            (if (<= (.y (+ (Transformation|GetWorldLocation _head_2) (* (* (Math|Vector|GetUpVector _head_2) (Variables|Default|GetdirectionMultiplier)) _newtrack_0))) (.y (Variables|Default|GetMoveLimit)))
              (goto _label)))
          (:3
            (if (<= (.z (+ (Transformation|GetWorldLocation _head_2) (* (* (Math|Vector|GetUpVector _head_2) (Variables|Default|GetdirectionMultiplier)) _newtrack_0))) (.z (Variables|Default|GetMoveLimit)))
              (goto _label))))))
    (else
      (Timeline|Timeline_0 Reverse))))

(event Custom|CustomEvent_0
  (bind _isa (Utilities|FlowControl|FlipFlop)
    (:A
      _)
    (:B
      _))
  (Variables|Default|SetisActivated _isa)
  (CallFunction|Trigger (Variables|Default|GetTriggerValue)))

(event EventBeginPlay
  (if (Variables|Default|GetisActivated)
    (CallFunction|PullHeadUp)))

(fn ConstructionScript)

(fn Trigger
  (params (InTriggerValue :type Integer))
  (if (CallFunction|IsTrigged InTriggerValue)
    (bind _output_get (Variables|Default|SetisActivated (not (Variables|Default|GetisActivated))))
    (if _output_get
      (CallFunction|PullHeadUp)
      (else
        (CallFunction|PullHeadDown)))))

(fn GetPullDirection
  (params (VectorUp :type Vector))
  (if (!= (.x VectorUp) 0.0)
    (return (Math|Float|Sign(Float) (.x VectorUp)))
    (elif (!= (.y VectorUp) 0.0)
      (return (* (.y VectorUp) 2.0))
      (elif (!= (.z VectorUp) 0.0)
        (return (* (.z VectorUp) 3.0))
        (else
          (return 0.0))))))