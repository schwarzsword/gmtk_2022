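; Double door actor locked by a rune, whose type sets the lock meshes and the light and Niagara colour in the construction script.
; Trigger opens or closes it via IsTrigged, toggling lock and light visibility and playing or reversing a timeline that swings both doors.
; Opening also activates Niagara and spawns a door effect from a timeline event.
; BeginPlay endlessly calls Trigger with alternating values on a fixed delay, apparently as a test loop.
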(event Custom|OpenDoors
  (Rendering|SetVisibility (Variables|Default|GetLock2) false false)
  (Components|Activation|Activate (Variables|Default|GetNiagara) true)
  (bind _alpha (Timeline|OpenCloseTimeLine PlayFromStart)
    (:Update
      (Transformation|SetRelativeRotation (Variables|Default|GetDoor1) (Math|Rotator|Lerp(Rotator) "0,-90.000000, 0" "0,-180.000000, 0" _alpha) false false)
      (Transformation|SetRelativeRotation (Variables|Default|GetDoor2) (Math|Rotator|Lerp(Rotator) "0,-90.000000, 0" "0, 0, 0" _alpha) false false))
    (:NewTrack_0
      (Niagara|SpawnSystematLocation "/Game/FX/FlipBook/NS_Door.NS_Door" (+ (Transformation|GetActorLocation) "0,0,50.000000")))))

(event Custom|CloseDoors
  (Rendering|SetVisibility (Variables|Default|GetLock2) true false)
  (bind _alpha (Timeline|OpenCloseTimeLine ReverseFromEnd)
    (:Update
      (Transformation|SetRelativeRotation (Variables|Default|GetDoor1) (Math|Rotator|Lerp(Rotator) "0,-90.000000, 0" "0,-180.000000, 0" _alpha) false false)
      (Transformation|SetRelativeRotation (Variables|Default|GetDoor2) (Math|Rotator|Lerp(Rotator) "0,-90.000000, 0" "0, 0, 0" _alpha) false false))
    (:NewTrack_0
      (Niagara|SpawnSystematLocation "/Game/FX/FlipBook/NS_Door.NS_Door" (+ (Transformation|GetActorLocation) "0,0,50.000000")))))

(event EventBeginPlay
  (|CallParentFunction)
  (Utilities|FlowControl|Delay 3.0 :!label _label)
  (CallFunction|Trigger)
  (Utilities|FlowControl|Delay 3.0)
  (CallFunction|Trigger 1)
  (goto _label))

(event Collision|EventActorBeginOverlap
  (params (OtherActor :type Actor%20Object%20Reference)))

(event EventTick
  (params (DeltaSeconds :type Float%20%28single-precision%29)))

(fn ConstructionScript
  (bind _lock2 (Variables|Default|GetLock2))
  (bind _lock1 (Variables|Default|GetLock1))
  (|CallParentFunction)
  (switch Utilities|FlowControl|Switch|SwitchonE_CubeSides (Variables|Default|GetNeededRune)
    (:NewEnumerator0
      (Components|StaticMesh|SetStaticMesh _lock2 "/Game/Static/rune_lock_1.rune_lock_1")
      (Components|StaticMesh|SetStaticMesh _lock1 "/Game/Static/rune_lock_1.rune_lock_1")
      (Rendering|Components|Light|SetLightColor (Variables|Default|GetPointLight) "(R=1.000000,G=0.841131,B=0.000000,A=1.000000)" true)
      (Effects|Components|ParticleSystem|SetColorParameter (Variables|Default|GetNiagara) "Color" "(R=1.000000,G=0.839216,B=0.000000,A=1.000000)"))
    (:NewEnumerator1
      (Components|StaticMesh|SetStaticMesh _lock2 "/Game/Static/rune_lock_2.rune_lock_2")
      (Components|StaticMesh|SetStaticMesh _lock1 "/Game/Static/rune_lock_2.rune_lock_2")
      (Rendering|Components|Light|SetLightColor (Variables|Default|GetPointLight) "(R=1.000000,G=0.000000,B=0.874510,A=1.000000)" true)
      (Effects|Components|ParticleSystem|SetColorParameter (Variables|Default|GetNiagara) "Color" "(R=1.000000,G=0.000000,B=0.874510,A=1.000000)"))
    (:NewEnumerator2
      (Components|StaticMesh|SetStaticMesh _lock2 "/Game/Static/rune_lock_3.rune_lock_3")
      (Components|StaticMesh|SetStaticMesh _lock1 "/Game/Static/rune_lock_3.rune_lock_3")
      (Rendering|Components|Light|SetLightColor (Variables|Default|GetPointLight) "(R=1.000000,G=0.043137,B=0.000000,A=1.000000)" true)
      (Effects|Components|ParticleSystem|SetColorParameter (Variables|Default|GetNiagara) "Color" "(R=1.000000,G=0.043137,B=0.000000,A=1.000000)"))
    (:NewEnumerator3
      (Components|StaticMesh|SetStaticMesh _lock2 "/Game/Static/rune_lock_4.rune_lock_4")
      (Components|StaticMesh|SetStaticMesh _lock1 "/Game/Static/rune_lock_4.rune_lock_4")
      (Rendering|Components|Light|SetLightColor (Variables|Default|GetPointLight) "(R=0.000000,G=1.000000,B=0.035294,A=1.000000)" true)
      (Effects|Components|ParticleSystem|SetColorParameter (Variables|Default|GetNiagara) "Color" "(R=0.000000,G=1.000000,B=0.035294,A=1.000000)"))
    (:NewEnumerator4
      (Components|StaticMesh|SetStaticMesh _lock2 "/Game/Static/rune_lock_5.rune_lock_5")
      (Components|StaticMesh|SetStaticMesh _lock1 "/Game/Static/rune_lock_5.rune_lock_5")
      (Rendering|Components|Light|SetLightColor (Variables|Default|GetPointLight) "(R=1.000000,G=1.000000,B=1.000000,A=1.000000)" true)
      (Effects|Components|ParticleSystem|SetColorParameter (Variables|Default|GetNiagara) "Color" "(R=1.000000,G=1.000000,B=1.000000,A=1.000000)"))
    (:NewEnumerator5
      (Components|StaticMesh|SetStaticMesh _lock2 "/Game/Static/rune_lock_6.rune_lock_6")
      (Components|StaticMesh|SetStaticMesh _lock1 "/Game/Static/rune_lock_6.rune_lock_6")
      (Rendering|Components|Light|SetLightColor (Variables|Default|GetPointLight) "(R=0.000000,G=0.007843,B=1.000000,A=1.000000)" true)
      (Effects|Components|ParticleSystem|SetColorParameter (Variables|Default|GetNiagara) "Color" "(R=0.000000,G=0.007843,B=1.000000,A=1.000000)"))))

(fn Trigger
  (params (InTriggerValue :type Integer))
  (if (CallFunction|IsTrigged InTriggerValue)
    (CallFunction|OpenDoors)
    (else
      (CallFunction|CloseDoors))))