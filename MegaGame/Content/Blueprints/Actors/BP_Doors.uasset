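; Door actor that slides its Cube component up to open and back down to close.
; Trigger passes its input value to IsTrigged and calls OpenDoors or CloseDoors based on the result.
; Both events drive OpenCloseTimeLine, playing from start or reversing from end, whose alpha lerps the cube's relative location along Z.
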(event Custom|OpenDoors
  (bind _alpha (Timeline|OpenCloseTimeLine PlayFromStart)
    (:Update
      (Transformation|SetRelativeLocation (Variables|Default|GetCube) (Math|Vector|Lerp(Vector) "0, 0, 0" "0, 0,250.000000" _alpha) false false))))

(event Custom|CloseDoors
  (bind _alpha (Timeline|OpenCloseTimeLine ReverseFromEnd)
    (:Update
      (Transformation|SetRelativeLocation (Variables|Default|GetCube) (Math|Vector|Lerp(Vector) "0, 0, 0" "0, 0,250.000000" _alpha) false false))))

(event EventBeginPlay
  (|CallParentFunction) ; This node is disabled and will not be called.\nDrag off pins to build functionality.
)

(event Collision|EventActorBeginOverlap
  (params (OtherActor :type Actor%20Object%20Reference)))

(event EventTick
  (params (DeltaSeconds :type Float%20%28single-precision%29)))

(fn ConstructionScript
  (|CallParentFunction))

(fn Trigger
  (params (InTriggerValue :type Integer))
  (if (CallFunction|IsTrigged InTriggerValue)
    (CallFunction|OpenDoors)
    (else
      (CallFunction|CloseDoors))))