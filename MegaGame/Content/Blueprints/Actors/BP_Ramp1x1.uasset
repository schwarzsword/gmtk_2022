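; BP_Ramp1x1 is a two-way ramp actor that moves the player cube between its lower and upper ends.
; An overlap at either end collider disables the cube's rotation check and calls its RampMove in slow mode, passing the ramp and direction-ordered marker positions.
; IsReady blocks re-triggering; the delayed logic that restores it and the rotation check is disconnected, so nothing live here resets them.
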(event OnComponentBeginOverlap(DownCollider)
  (params (OverlappedComponent :type Primitive%20Component%20Object%20Reference) (OtherActor :type Actor%20Object%20Reference) (OtherComp :type Primitive%20Component%20Object%20Reference) (OtherBodyIndex :type Integer) (bFromSweep :type Boolean) (SweepResult :type Hit%20Result%20Structure%20%28by%20ref%29))
  (bind _asbp_player_cube (Utilities|Casting|CastToBP_PlayerCube OtherActor))
  (if (Variables|Default|GetIsReady)
    (Variables|Default|SetIsReady false)
    (Variables|/Game/Blueprints/Characters/BP_PlayerCube.BP_PlayerCube_C|SetRotationCheckEnabled _asbp_player_cube false)
    (Default|RampMove _asbp_player_cube (Transformation|GetWorldLocation (Variables|Default|GetDownPoint)) (Transformation|GetWorldLocation (Variables|Default|GetUpPoint)) true self (Transformation|GetWorldLocation (Variables|Default|GetUpLastPoint)) (Transformation|GetWorldLocation (Variables|Default|GetDownLastPoint)))))

(event OnComponentBeginOverlap(UpCollider)
  (params (OverlappedComponent :type Primitive%20Component%20Object%20Reference) (OtherActor :type Actor%20Object%20Reference) (OtherComp :type Primitive%20Component%20Object%20Reference) (OtherBodyIndex :type Integer) (bFromSweep :type Boolean) (SweepResult :type Hit%20Result%20Structure%20%28by%20ref%29))
  (bind _asbp_player_cube (Utilities|Casting|CastToBP_PlayerCube OtherActor))
  (if (Variables|Default|GetIsReady)
    (Variables|Default|SetIsReady false)
    (Variables|/Game/Blueprints/Characters/BP_PlayerCube.BP_PlayerCube_C|SetRotationCheckEnabled _asbp_player_cube false)
    (Default|RampMove _asbp_player_cube (Transformation|GetWorldLocation (Variables|Default|GetUpPoint)) (Transformation|GetWorldLocation (Variables|Default|GetDownPoint)) true self (Transformation|GetWorldLocation (Variables|Default|GetDownLastPoint)) (Transformation|GetWorldLocation (Variables|Default|GetUpLastPoint)))))

(fn ConstructionScript)