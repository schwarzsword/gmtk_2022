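; BP_CubeHP tracks the cube's health as a max and current HP pair, with functions to remove one point, add one capped at max, or remove all.
; Health changes notify the first top-level WBP_HealthBar widget found through a class search to increase or decrease its display.
; Removing all HP loops the single-point removal, and reaching zero calls the EDRestart dispatcher and prints a debug string.
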(event EventBeginPlay)

(event EventTick
  (params (DeltaSeconds :type Float%20%28single-precision%29)))

(fn FunctionRemoveHP
  (Variables|Default|SetHealth (Utilities|Struct|MakeST_HP (.maxhp (Variables|Default|GetHealth)) (- (.realhp (Variables|Default|GetHealth)) 1)))
  (bind _foundwidgets (Widget|GetAllWidgetsOfClass "/Game/UI/WBP_HealthBar.WBP_HealthBar_C" true))
  (Default|EventDecreaseHP (Utilities|Array|Get(acopy) _foundwidgets))
  (if (== (.realhp (Variables|Default|GetHealth)) 0)
    (Default|CallEDRestart)
    (Development|PrintString "Hello")))

(fn FunctionAddHP
  (if (<= (.maxhp (Variables|Default|GetHealth)) (.realhp (Variables|Default|GetHealth)))
    (Variables|Default|SetHealth (Utilities|Struct|MakeST_HP (.maxhp (Variables|Default|GetHealth)) (.maxhp (Variables|Default|GetHealth))))
    (else
      (Variables|Default|SetHealth (Utilities|Struct|MakeST_HP (.maxhp (Variables|Default|GetHealth)) (+ (.realhp (Variables|Default|GetHealth)) 1)))
      (bind _foundwidgets (Widget|GetAllWidgetsOfClass "/Game/UI/WBP_HealthBar.WBP_HealthBar_C" true))
      (Default|EventIncreaseHP (Utilities|Array|Get(acopy) _foundwidgets)))))

(fn FunctionRemoveAllHP
  (bind _output_get (LocalVariables|SetCounter (- (.realhp (Variables|Default|GetHealth)) 1)))
  (for _index (range 0 _output_get)
    (CallFunction|FunctionRemoveHP)))